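; Pinball game mode Blueprint that handles scoring and lost balls.
; AddScore adds the given points to the score held in BP_PinballGameState.
; OnBallLost checks that game state's remaining balls, then either decrements the count and calls SpawnBall, or only prints "Game Over" when none remain.
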(event `/Game/Blueprints/BPI_ScoreReceiver.AddScore`
  (params (Points :type "Float (double-precision)"))
  (bind _asbp_pinball_game_state (cast `/Game/Blueprints/BP_PinballGameState` (`GameplayStatics.GetGameState`)))
  (`/Game/Blueprints/BP_PinballGameState.SetScore` _asbp_pinball_game_state (+ Points (`/Game/Blueprints/BP_PinballGameState.Score` _asbp_pinball_game_state))))

(event `self.OnBallLost`
  (bind _asbp_pinball_game_state (cast `/Game/Blueprints/BP_PinballGameState` (`GameplayStatics.GetGameState`)))
  (if (<= (`/Game/Blueprints/BP_PinballGameState.BallsRemaining` _asbp_pinball_game_state) 0)
    (`KismetSystemLibrary.PrintString` "Game Over")
    (else
      (`/Game/Blueprints/BP_PinballGameState.SetBalls` _asbp_pinball_game_state (- (`/Game/Blueprints/BP_PinballGameState.BallsRemaining` _asbp_pinball_game_state) 1))
      (`/Game/Blueprints/BPI_GameMode.SpawnBall`))))

(fn `UserConstructionScript`
  (`parent.UserConstructionScript`))