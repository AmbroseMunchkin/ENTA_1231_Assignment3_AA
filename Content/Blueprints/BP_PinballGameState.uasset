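; Pinball game state Blueprint that holds the current score and the number of balls remaining.
; SetScore and SetBalls events store the new value, then broadcast it through the OnScoreChanged or OnBallsChanged dispatcher so listeners can react.
; Each setter also prints the new value as a string, and the Blueprint has no BeginPlay, Tick or construction logic.
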(event `self.ReceiveBeginPlay`)

(event `SetScore`
  (params (NewScore :type "Float (double-precision)"))
  (bind _output_get (set `self.Score` NewScore))
  (`self.OnScoreChanged` _output_get)
  (`KismetSystemLibrary.PrintString` (`KismetStringLibrary.Conv_DoubleToString` (`self.Score`))))

(event `SetBalls`
  (params (NewBalls :type Integer))
  (bind _output_get (set `self.BallsRemaining` NewBalls))
  (`self.OnBallsChanged` _output_get)
  (`KismetSystemLibrary.PrintString` (`KismetStringLibrary.Conv_IntToString` (`self.BallsRemaining`))))

(fn `UserConstructionScript`)