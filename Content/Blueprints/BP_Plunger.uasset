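; Pinball plunger actor that pulls back while charging and launches the ball with force based on the charge.
; Charge runs a timeline that moves the plunger toward its end position, recording alpha and position; Release stops it and animates back from that point.
; When a BPI_PinballReactive actor stops overlapping the box, it receives an impulse away from the plunger actor, scaled by MaxForce and recorded charge.
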(event `Charge`
  (bind (_direction _charge_alpha) (`Timeline|Timeline` :!via `PlayFromStart` :!label _label)
    (:`Update`
      (set `self.ChargeTime` _charge_alpha)
      (bind _returnvalue (`KismetMathLibrary.VLerp` (`self.StartPos`) (`self.EndPos`) _charge_alpha))
      (set `self.UpdatedPos` _returnvalue)
      (`SceneComponent.K2_SetRelativeLocation` (`self.Plunger`) _returnvalue false false))))

(event `Release`
  (`|ExecutionSequence`
    (:`then_0`
      (goto _label :!via `Stop`))
    (:`then_1`
      (bind (_direction _charge_alpha) (`Timeline|Timeline_0` :!via `PlayFromStart`)
        (:`Update`
          (`SceneComponent.K2_SetRelativeLocation` (`self.Plunger`) (`KismetMathLibrary.VLerp` (`self.UpdatedPos`) (`self.StartPos`) _charge_alpha) false false))))))

(event `self.Box.OnComponentEndOverlap`
  (params (OverlappedComponent :type "PrimitiveComponent Object Reference") (OtherActor :type "Actor Object Reference") (OtherComp :type "PrimitiveComponent Object Reference") (OtherBodyIndex :type Integer))
  (bind _asbpi_pinball_reactive (cast `/Game/Blueprints/BPI_PinballReactive` OtherActor))
  (`/Game/Blueprints/BPI_PinballReactive.PinballImpulseEvent` _asbpi_pinball_reactive (* (* (`self.MaxForce`) (`self.ChargeTime`)) (`KismetMathLibrary.Normal` (- (`SceneComponent.K2_GetComponentLocation` OtherComp) (`self.K2_GetActorLocation`))))))

(fn `UserConstructionScript`)