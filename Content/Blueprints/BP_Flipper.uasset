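; A flipper actor that swings its Flipper component around the yaw axis when activated, like a pinball paddle.
; On BeginPlay it derives an end rotation 90 degrees from zero, with the sign picked by its Direction enum.
; Activation plays a Timeline that lerps the relative rotation from start to end, and deactivation reverses it to swing back.
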(event `OnActivate`
  (bind (_direction _rotation) (`Timeline|Timeline` :!label _label)
    (:`Update`
      (`SceneComponent.K2_SetRelativeRotation` (`self.Flipper`) (`KismetMathLibrary.RLerp` (`self.StartRot`) (`self.EndRot`) _rotation) false false))))

(event `OnDeactivate`
  (goto _label :!via `Reverse`))

(event `self.ReceiveBeginPlay`
  (bind _output_get (set `self.StartRot` (struct)))
  (set `self.EndRot` (`KismetMathLibrary.ComposeRotators` _output_get (`KismetMathLibrary.SelectRotator` (struct :`Yaw` -90.0) (struct :`Yaw` 90.0) (`|EnumEquality` (`self.Direction`) "NewEnumerator1")))))

(fn `UserConstructionScript`)