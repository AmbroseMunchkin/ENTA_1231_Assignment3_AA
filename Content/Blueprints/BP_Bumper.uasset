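; Pinball bumper that knocks reactive objects away and awards score.
; On capsule overlap, it sends an outward impulse through BPI_PinballReactive, then adds points via GM_Pinball_Score for those objects only.
; Any overlap also plays a timeline that lerps the Mechanism and spawns a hugely scaled NG_Nothing effect on every update, aimed away from the bumper.
; Ending overlap stops the timeline and snaps the Mechanism back to its start.
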(event `self.Capsule.OnComponentBeginOverlap`
  (params (OverlappedComponent :type "PrimitiveComponent Object Reference") (OtherActor :type "Actor Object Reference") (OtherComp :type "PrimitiveComponent Object Reference") (OtherBodyIndex :type Integer) (bFromSweep :type Boolean) (SweepResult :type "HitResult Structure (by ref)"))
  (bind _returnvalue (`self.K2_GetActorLocation`))
  (bind _returnvalue_2 (`SceneComponent.K2_GetComponentLocation` OtherComp))
  (`|ExecutionSequence`
    (:`then_0`
      ; Applies Force
      (bind _asbpi_pinball_reactive (cast `/Game/Blueprints/BPI_PinballReactive` OtherActor))
      (`/Game/Blueprints/BPI_PinballReactive.PinballImpulseEvent` _asbpi_pinball_reactive (* (`self.BumperStrength`) (`KismetMathLibrary.Normal` (- _returnvalue_2 _returnvalue))))
      ; Adds score
      (bind _asgm_pinball_score (cast `/Game/Blueprints/GM_Pinball_Score` (`GameplayStatics.GetGameMode`)))
      (`/Game/Blueprints/BPI_ScoreReceiver.AddScore` _asgm_pinball_score (`self.ScoreValue`)))
    (:`then_1`
      ; play anim
      (bind (_direction _charge_alpha) (`Timeline|Timeline` :!label _label)
        (:`Update`
          (`SceneComponent.K2_SetRelativeLocation` (`self.Mechanism`) (`KismetMathLibrary.VLerp` (`self.StartPos`) (`self.EndPos`) _charge_alpha) false false)
          (`NiagaraFunctionLibrary.SpawnSystemAtLocation` "/Game/Blueprints/NG_Nothing.NG_Nothing" _returnvalue_2 (`KismetMathLibrary.FindLookAtRotation` _returnvalue _returnvalue_2) (50000.0 50000.0 500000.0)))))))

(event `self.Capsule.OnComponentEndOverlap`
  (params (OverlappedComponent :type "PrimitiveComponent Object Reference") (OtherActor :type "Actor Object Reference") (OtherComp :type "PrimitiveComponent Object Reference") (OtherBodyIndex :type Integer))
  (`|ExecutionSequence`
    (:`then_0`
      (goto _label :!via `Stop`))
    (:`then_1`
      (`SceneComponent.K2_SetRelativeLocation` (`self.Mechanism`) (`self.StartPos`) false false))))

(fn `UserConstructionScript`)